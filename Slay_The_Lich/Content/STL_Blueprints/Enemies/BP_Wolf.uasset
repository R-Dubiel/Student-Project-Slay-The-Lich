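; BP_Wolf is a wolf enemy that rests, roams around its spawn point or chases the player.
; A delay-driven BeginPlay loop switches modes by a simple distance check and issues AI moves until the wolf dies.
; Tick plays a jump-bite montage at close range, pausing movement; AttackNear applies damage but isn't called here.
; AnyDamage updates the life-bar widget and, at zero life, stops movement and disables collision.
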(event EventBeginPlay
  (CallFunction|SetPlayerState)
  (CallFunction|UpdateLifeBar)
  (Variables|Default|SetStartingLocation (Transformation|GetActorLocation))
  (switch Utilities|FlowControl|Switch|SwitchonBehaviour_wolf (Variables|EnemyVariables|GetMode) :!label _label
    (:NewEnumerator0
      (bind _returnvalue (CallFunction|SeePlayer))
      (if _returnvalue
        (Variables|EnemyVariables|SetMode "NewEnumerator2" :!label _label_2)
        (Utilities|FlowControl|Delay 0.5)
        (else
          (Variables|EnemyVariables|SetMode "NewEnumerator0")
          (Utilities|FlowControl|Delay 0.5))))
    (:NewEnumerator1
      (bind _returnvalue_2 (CallFunction|SeePlayer))
      (if _returnvalue_2
        (goto _label_2)
        (else
          (AI|AIMoveTo self (.RandomLocation (AI|Navigation|GetRandomReachablePointinRadius (Variables|Default|GetStartingLocation) (Math|Float|Clamp(Float) (Variables|Default|GetRadius) 5e+02 2.5e+03) 0 0)) 0 5.0 false
            (:then
              (Utilities|FlowControl|Delay 2.5 :!label _label_3))))))
    (:NewEnumerator2
      (bind _returnvalue_3 (CallFunction|SeePlayer))
      (if _returnvalue_3
        (AI|AIMoveTo self "0, 0, 0" (Game|GetPlayerCharacter 0) 5.0 false
          (:then
            (Utilities|FlowControl|Delay 0.2)))
        (else
          (Variables|EnemyVariables|SetMode "NewEnumerator1")
          (goto _label_3)))))
  (if (not (Variables|EnemyVariables|GetHas%20Died))
    (goto _label)))

(event EventTick
  (params (DeltaSeconds :type Float%20%28single-precision%29))
  (CallFunction|SetPlayerState)
  (if (not (or (Variables|Character|GetPlayer%20Has%20Died) (Variables|EnemyVariables|GetHas%20Died)))
    (if (and (< (Transformation|GetDistanceTo (Game|GetPlayerCharacter 0)) 1.5e+02) (not (CallFunction|IsWolfAttacking)))
      (Components|Activation|Deactivate (Variables|Character|GetCharacterMovement))
      (Animation|Montage|PlayMontage (Variables|Character|GetMesh) "/Game/AnimalVarietyPack/Wolf/Animations/ANIM_Wolf_JumpBite_Montage.ANIM_Wolf_JumpBite_Montage"
        (:OnCompleted
          (Components|Activation|Activate (Variables|Character|GetCharacterMovement) false))))))

(event Game|Damage|EventAnyDamage
  (params (Damage :type Float%20%28single-precision%29) (DamageType :type Damage%20Type%20Object%20Reference) (InstigatedBy :type Controller%20Object%20Reference) (DamageCauser :type Actor%20Object%20Reference))
  (bind _charactermovement (Variables|Character|GetCharacterMovement))
  (Variables|EnemyVariables|SetLife (Math|Float|Clamp(Float) (- (Variables|EnemyVariables|GetLife) Damage) 0.0 1e+02))
  (CallFunction|UpdateLifeBar)
  (Variables|EnemyVariables|SetHas%20Died (== (Variables|EnemyVariables|GetLife) 0.0))
  (if (Variables|EnemyVariables|GetHas%20Died)
    (Components|Movement|StopMovementImmediately _charactermovement)
    (Components|Activation|Deactivate _charactermovement)
    (Collision|SetActorEnableCollision false)))

(fn ConstructionScript)

(fn AttackNear
  (Game|Damage|ApplyDamage (Game|GetPlayerCharacter 0) 1e+01 0 0))

(fn IsWolfAttacking
  (return (Animation|Montage|MontageIsPlaying (Components|SkeletalMesh|GetAnimInstance (Variables|Character|GetMesh)) "/Game/AnimalVarietyPack/Wolf/Animations/ANIM_Wolf_JumpBite_Montage.ANIM_Wolf_JumpBite_Montage")))

(fn SetPlayerState
  (bind _asbp_top_down_character (Utilities|Casting|CastToBP_TopDownCharacter (Game|GetPlayerCharacter 0)))
  (Variables|Character|SetPlayer%20Has%20Died (Variables|/Game/TopDown/Blueprints/BP_TopDownCharacter.BP_TopDownCharacter_C|GetHas%20Died _asbp_top_down_character)))

(fn UpdateLifeBar
  (bind _aswb_wolf_life_bar (Utilities|Casting|CastToWB_Wolf_Life_Bar (UserInterface|GetUserWidgetObject (Variables|Default|GetLifeBar))))
  (Variables|/Game/STL_Blueprints/Enemies/WB_Wolf_Life_Bar.WB_Wolf_Life_Bar_C|SetLife _aswb_wolf_life_bar (/ (Variables|EnemyVariables|GetLife) 1e+02)))

(fn SeePlayer
  (return (< (Transformation|GetDistanceTo (Game|GetPlayerCharacter 0)) 2e+03)))