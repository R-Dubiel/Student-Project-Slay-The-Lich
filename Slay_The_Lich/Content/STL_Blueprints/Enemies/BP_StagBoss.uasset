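; Stag boss enemy driven by a looping behaviour-mode state machine that starts fighting when the player is within range.
; It retreats to random points, then picks melee or a high-speed charge by distance, returning to defense after melee.
; Tick triggers close-range antler montages with distance-checked damage.
; Damage updates the life bar and handles death, though the same Dead flag is overwritten each tick by the player's death state.
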(event EventBeginPlay
  (bind _charactermovement (Variables|Character|GetCharacterMovement))
  (bind _charactermovement_2 (Variables|Character|GetCharacterMovement))
  (CallFunction|SetPlayerState)
  (switch Utilities|FlowControl|Switch|SwitchonBehaviourModes (Variables|Default|GetBehaviourMode) :!label _label
    (:NewEnumerator0
      (bind _returnvalue (CallFunction|SeePlayer))
      (if _returnvalue
        (Variables|Default|SetBehaviourMode "NewEnumerator3" :!label _label_2)
        (else
          (Variables|Default|SetBehaviourMode "NewEnumerator0"))))
    (:NewEnumerator1
      (Variables|/Script/Engine.CharacterMovementComponent|SetMaxWalkSpeed _charactermovement 5e+02)
      (AI|AIMoveTo self "0, 0, 0" (Game|GetPlayerCharacter 0) 5.0 false
        (:then
          (Utilities|FlowControl|Delay 1.5)
          (goto _label_2))))
    (:NewEnumerator2
      (Utilities|FlowControl|Delay 0.5)
      (Variables|/Script/Engine.CharacterMovementComponent|SetMaxWalkSpeed _charactermovement_2 4e+03)
      (AI|AIMoveTo self "0, 0, 0" (Game|GetPlayerCharacter 0) 5.0 false
        (:then
          (Utilities|FlowControl|Delay 0.8)
          (Variables|/Script/Engine.CharacterMovementComponent|SetMaxWalkSpeed _charactermovement_2 5e+02)
          (Variables|Default|SetBehaviourMode "NewEnumerator1" :!label _label_3))))
    (:NewEnumerator3
      (Variables|/Script/Engine.CharacterMovementComponent|SetMaxWalkSpeed _charactermovement 1e+03)
      (AI|AIMoveTo self (.RandomLocation (AI|Navigation|GetRandomReachablePointinRadius (Transformation|GetActorLocation) (Variables|Default|GetRadius) 0 0)) 0 5.0 false
        (:then
          (Utilities|FlowControl|Delay 0.5)
          (Variables|/Script/Engine.CharacterMovementComponent|SetMaxWalkSpeed _charactermovement 2.5e+02)
          (if (< (Transformation|GetDistanceTo (Game|GetPlayerCharacter 0)) 5e+02)
            (goto _label_3)
            (else
              (Variables|Default|SetBehaviourMode "NewEnumerator2"))))))
    (:NewEnumerator5
      (Utilities|FlowControl|Delay 1.0)
      (goto _label_2)))
  (Utilities|FlowControl|Delay 0.5)
  (goto _label))

(event EventTick
  (params (DeltaSeconds :type Float%20%28single-precision%29))
  (CallFunction|SetPlayerState)
  (if (not (Variables|Default|GetDead?))
    (if (and (< (Transformation|GetDistanceTo (Game|GetPlayerCharacter 0)) 1.5e+02) (not (CallFunction|IsAttacking)))
      (Components|Activation|Deactivate (Variables|Character|GetCharacterMovement))
      (Animation|Montage|PlayMontage (Variables|Character|GetMesh) "/Game/AnimalVarietyPack/DeerStagAndDoe/Animations/ANIM_DeerStag_AntlersAttack_Montage.ANIM_DeerStag_AntlersAttack_Montage"
        (:then
          (CallFunction|DamageHitbox)
          (Components|Activation|Activate (Variables|Character|GetCharacterMovement) false))))))

(event Game|Damage|EventAnyDamage
  (params (Damage :type Float%20%28single-precision%29) (DamageType :type Damage%20Type%20Object%20Reference) (InstigatedBy :type Controller%20Object%20Reference) (DamageCauser :type Actor%20Object%20Reference))
  (bind _charactermovement (Variables|Character|GetCharacterMovement))
  (Variables|Default|SetHealth (Math|Float|Clamp(Float) (- (Variables|Default|GetHealth) Damage) 0.0 1e+02))
  (CallFunction|SetHealth)
  (Variables|Default|SetDead? (== (Variables|Default|GetHealth) 0.0))
  (if (Variables|Default|GetDead?)
    (Components|Movement|StopMovementImmediately _charactermovement)
    (Components|Activation|Deactivate _charactermovement)
    (Collision|SetActorEnableCollision false)
    (Animation|Montage|PlayMontage (Variables|Character|GetMesh) "/Game/AnimalVarietyPack/DeerStagAndDoe/Animations/ANIM_DeerStag_Death_Montage.ANIM_DeerStag_Death_Montage")))

(fn ConstructionScript)

(fn UpdatePatrolPoint
  (bind _self self)
  (bind _outactors (Actor|GetAllActorsOfClass "/Game/STL_Blueprints/Enemies/EnemyPatrolPoint_BP.EnemyPatrolPoint_BP_C"))
  (for _array_element _outactors
    (if (< (Transformation|GetDistanceTo _array_element _self) (Transformation|GetDistanceTo (Variables|Default|GetPatrolPointRef) _self))
      (Variables|Default|SetPatrolPointRef _array_element))))

(fn SetPlayerState
  (bind _asbp_top_down_character (Utilities|Casting|CastToBP_TopDownCharacter (Game|GetPlayerCharacter 0)))
  (Variables|Default|SetDead? (Variables|/Game/TopDown/Blueprints/BP_TopDownCharacter.BP_TopDownCharacter_C|GetHas%20Died _asbp_top_down_character)))

(fn SetHealth
  (bind _aswb_wolf_life_bar (Utilities|Casting|CastToWB_Wolf_Life_Bar (UserInterface|GetUserWidgetObject (Variables|Default|GetLifeBar1))))
  (Variables|/Game/STL_Blueprints/Enemies/WB_Wolf_Life_Bar.WB_Wolf_Life_Bar_C|SetLife _aswb_wolf_life_bar (/ (Variables|Default|GetHealth) 1e+02)))

(fn SeePlayer
  (return (< (Transformation|GetDistanceTo (Game|GetPlayerCharacter 0)) 2e+03)))

(fn DamageHitbox
  (bind _returnvalue (Game|GetPlayerCharacter 0))
  (if (< (Transformation|GetDistanceTo _returnvalue) 2e+02)
    (Game|Damage|ApplyDamage _returnvalue (Variables|Default|GetCurrent%20Enemy%20Damage) 0 0)
    (Animation|PlayAnimMontage "/Game/AnimalVarietyPack/DeerStagAndDoe/Animations/ANIM_DeerStag_AntlersAttack_Montage.ANIM_DeerStag_AntlersAttack_Montage" 1.0 "None")))

(fn IsAttacking
  (return (Animation|Montage|MontageIsPlaying (Components|SkeletalMesh|GetAnimInstance (Variables|Character|GetMesh)) "/Game/AnimalVarietyPack/DeerStagAndDoe/Animations/ANIM_DeerStag_AntlersAttack_Montage.ANIM_DeerStag_AntlersAttack_Montage")))