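; BP_Fox is a fox enemy that patrols around its spawn point, then chases and attacks the player once it sees them or takes damage.
; Tick drives AIMoveTo to random points or the target, and reaching the player triggers a range-checked, delayed attack montage.
; A separate attack event damages the player through a forward sphere overlap.
; Damage updates a reused wolf life-bar widget, and zero life plays a death animation before destroying the actor.
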(event OnSeePawn(PawnSensing)
  (params (Pawn :type Pawn%20Object%20Reference))
  ;[1 1 1] Sense the player
  (Variables|Character|GetPlayer%20Target
    (:then)
    (:else
      (Variables|Character|SetPlayer%20Target Pawn))))

(event Custom|Chase%20Player
  (params (Target%20Actor :type Pawn%20Object%20Reference))
  ;[1 1 1] Chase Player
  (AI|AIMoveTo self "0, 0, 0" Target%20Actor (Variables|EnemyVariables-Settings|GetAcceptance%20Radius%20From%20Player) true
    (:OnSuccess
      (CallFunction|CanAttack?))))

(event Custom|Patrol
  ;[1 1 1] Enemy Patrol
  (if (> (Utilities|Time|GetTimeSeconds) (+ (Variables|Default|GetTime%20since%20patrol) 4.0))
    (AI|AIMoveTo self (.RandomLocation (AI|Navigation|GetRandomReachablePointinRadius (Variables|Default|GetStartingLocation) 2e+03 0 0)) 0 5.0 false
      (:then
        (Variables|Default|SetTime%20since%20patrol (Utilities|Time|GetTimeSeconds))))))

(event Custom|CanAttack?
  ;[1 1 1] Initialize Attack if valid
  (bind _dead (Class|IntBPTopDownCharacter|PlayerHasDied?(Message) (Variables|Character|GetPlayer%20Target)))
  (bind _returnvalue (CallFunction|PlayerinRange))
  (if (Math|Boolean|ANDBoolean _returnvalue (not _dead) (not (Variables|EnemyVariables-Current|GetHas%20Died)) (not (Variables|EnemyVariables-Current|GetIs%20Attacking)))
    (Variables|EnemyVariables-Current|SetIs%20Attacking true)
    (Utilities|FlowControl|Delay 0.8)
    (Animation|Montage|PlayMontage (Variables|Character|GetMesh) (Variables|Default|GetMontage%20to%20Play)
      (:OnCompleted
        (Variables|EnemyVariables-Current|SetIs%20Attacking false)))))

(event Game|Damage|EventAnyDamage
  (params (Damage :type Float%20%28single-precision%29) (DamageType :type Damage%20Type%20Object%20Reference) (InstigatedBy :type Controller%20Object%20Reference) (DamageCauser :type Actor%20Object%20Reference))
  (bind _charactermovement (Variables|Character|GetCharacterMovement))
  ;[1 1 1] Take Damage
  (Variables|Character|SetPlayer%20Target (Game|GetPlayerCharacter 0))
  (Variables|EnemyVariables-Current|SetLife (Math|Float|Clamp(Float) (- (Variables|EnemyVariables-Current|GetLife) Damage) 0.0 (Variables|Default|GetMaxLife)))
  (CallFunction|UpdateLifeBar)
  (if (== (Variables|EnemyVariables-Current|GetLife) 0.0)
    (Variables|EnemyVariables-Current|SetHas%20Died true)
    (Components|Movement|StopMovementImmediately _charactermovement)
    (Components|Activation|Deactivate _charactermovement)
    (Collision|SetActorEnableCollision false)
    (Components|Animation|PlayAnimation (Variables|Character|GetMesh) "/Game/AnimalVarietyPack/Fox/Animations/ANIM_Fox_Death.ANIM_Fox_Death" false)
    (Utilities|FlowControl|Delay 4.0)
    (Actor|DestroyActor)))

(event EventBeginPlay
  ;[1 1 1] Initialize the enemy
  (Variables|Default|SetMaxLife (Variables|EnemyVariables-Current|GetLife))
  (CallFunction|UpdateLifeBar)
  (Variables|Default|SetStartingLocation (Transformation|GetActorLocation)))

(event EventCurrentEnemyAttacks
  ;[1 1 1] Deal Damage
  (bind _outactors (Collision|SphereOverlapActors (+ (Transformation|GetActorLocation) (* (Transformation|GetActorForwardVector) (Variables|EnemyVariables-Settings|GetCurrent%20Enemy%20Attack%20-%20Forward%20Range))) (Variables|EnemyVariables-Settings|GetCurrent%20Enemy%20Attack%20-%20Sphere%20Radius) (Utilities|Array|MakeArray "ObjectTypeQuery3") "/Game/TopDown/Blueprints/BP_TopDownCharacter.BP_TopDownCharacter_C"))
  (for _array_element _outactors
    (Game|Damage|ApplyDamage _array_element (Variables|EnemyVariables-Settings|GetCurrent%20Enemy%20Damage) 0 0)))

(event EventTick
  (params (DeltaSeconds :type Float%20%28single-precision%29))
  ;[1 1 1] Tick Logic
  (if (not (Variables|EnemyVariables-Current|GetHas%20Died))
    (bind _player_target (Variables|Character|GetPlayer%20Target)
      (:then
        (CallFunction|ChasePlayer _player_target))
      (:else
        (CallFunction|Patrol)))))

(fn ConstructionScript)

(fn UpdateLifeBar
  (bind _aswb_wolf_life_bar (Utilities|Casting|CastToWB_Wolf_Life_Bar (UserInterface|GetUserWidgetObject (Variables|Default|GetLifeBar))))
  (Variables|/Game/STL_Blueprints/Enemies/WB_Wolf_Life_Bar.WB_Wolf_Life_Bar_C|SetLife _aswb_wolf_life_bar (/ (Variables|EnemyVariables-Current|GetLife) (Variables|Default|GetMaxLife))))

(fn PlayerinRange
  (return (< (Transformation|GetDistanceTo (Variables|Character|GetPlayer%20Target)) (Variables|EnemyVariables-Settings|GetCurrent%20Enemy%20Attack%20-%20Distance))))

(fn HasDied?
  (return (Variables|EnemyVariables-Current|GetHas%20Died)))