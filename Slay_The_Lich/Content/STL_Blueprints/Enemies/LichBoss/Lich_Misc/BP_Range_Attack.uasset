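; BP_Range_Attack is the Lich boss's ranged attack actor, which damages the player on contact.
; On sphere overlap, it checks that the player character has not died and that the other actor has the Player tag.
; A valid hit applies damage credited to the instigator and spawns an explosion emitter at the actor's location.
; Any overlap destroys the actor, whether or not it deals damage.
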(event OnComponentBeginOverlap(Sphere)
  (params (OverlappedComponent :type Primitive%20Component%20Object%20Reference) (OtherActor :type Actor%20Object%20Reference) (OtherComp :type Primitive%20Component%20Object%20Reference) (OtherBodyIndex :type Integer) (bFromSweep :type Boolean) (SweepResult :type Hit%20Result%20Structure%20%28by%20ref%29))
  (bind (_bblockinghit _binitialoverlap _time _distance _location _impactpoint _normal _impactnormal _physmat _hitactor) (Collision|BreakHitResult SweepResult))
  (bind _dead (Class|IntBPTopDownCharacter|PlayerHasDied?(Message) (Game|GetPlayerCharacter 0)))
  (if (and (not _dead) (Actor|ActorHasTag OtherActor "Player"))
    (Variables|Default|SetImpact%20Point _impactpoint)
    (Game|Damage|ApplyDamage _hitactor (Variables|Default|GetBase%20Damage) 0 (Game|GetInstigator))
    (CallFunction|DoExplosion (Variables|Default|GetEmitter%20Template) (Transformation|GetActorLocation) (Variables|Default|GetScale))
    (Actor|DestroyActor)
    (else
      (Actor|DestroyActor))))

(event Custom|Do%20Explosion
  (params (EmitterTemplate :type Particle%20System%20Object%20Reference) (Location :type Vector) (Scale :type Vector))
  (Effects|SpawnEmitteratLocation EmitterTemplate Location "0, 0, 0" Scale))

(event EventBeginPlay)

(event Collision|EventActorBeginOverlap
  (params (OtherActor :type Actor%20Object%20Reference)))

(event EventTick
  (params (DeltaSeconds :type Float%20%28single-precision%29)))

(fn ConstructionScript)